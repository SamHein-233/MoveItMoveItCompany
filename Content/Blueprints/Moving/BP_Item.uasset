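; BP_Item is a holdable item with a Cube component that can be picked up, dropped and used.
; Pickup turns off the cube's collision and attaches the item to the ItemSocket_L socket on the supplied parent.
; Drop detaches the cube in world space, restores collision and enables physics, with a zero force that adds no throw.
; PrimaryAction is a stub that, like the other events, prints a debug string.
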(event `Pickup`
  (params (Parent :type "SceneComponent Object Reference"))
  (`KismetSystemLibrary.PrintString` "Pickup")
  (`PrimitiveComponent.SetCollisionEnabled` (`self.Cube`) "NoCollision")
  (`self.K2_AttachToComponent` Parent "ItemSocket_L" "SnapToTarget" "SnapToTarget" "KeepRelative"))

(event `Drop`
  (bind _cube (`self.Cube`))
  (`KismetSystemLibrary.PrintString` "Drpo")
  (`SceneComponent.K2_DetachFromComponent` _cube "KeepWorld" "KeepWorld" "KeepRelative" true)
  (`PrimitiveComponent.SetCollisionEnabled` _cube "QueryAndPhysics")
  (`PrimitiveComponent.SetSimulatePhysics` _cube true)
  (`PrimitiveComponent.AddForce` _cube (0.0 0.0 0.0) "None" false))

(event `PrimaryAction`
  (`KismetSystemLibrary.PrintString` "PRimary"))

(fn `UserConstructionScript`)