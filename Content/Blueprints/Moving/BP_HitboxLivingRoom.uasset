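; Trigger hitbox that turns a delivered item into visible, solid living room furniture.
; When a BP_Item overlaps the Box, it finds the BP_LivingRoom actor by class and shows its root, propagating visibility to all children.
; It then destroys the item and enables query and physics collision on the living room's table and armchair meshes, with debug prints along the way.
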(event `self.Box.OnComponentBeginOverlap`
  (params (OverlappedComponent :type "PrimitiveComponent Object Reference") (OtherActor :type "Actor Object Reference") (OtherComp :type "PrimitiveComponent Object Reference") (OtherBodyIndex :type Integer) (bFromSweep :type Boolean) (SweepResult :type "HitResult Structure (by ref)"))
  (cast `/Game/Blueprints/Moving/BP_Item` OtherActor)
  (`KismetSystemLibrary.PrintString` "ITEM PLACED!")
  (bind _returnvalue (`GameplayStatics.GetActorOfClass` "/Game/Blueprints/Moving/BP_LivingRoom.BP_LivingRoom_C"))
  (`SceneComponent.SetVisibility` (`/Game/Blueprints/Moving/BP_LivingRoom.DefaultSceneRoot` _returnvalue) true true)
  (`KismetSystemLibrary.PrintString` "Visibilty changed!")
  (`self.K2_DestroyActor` OtherActor)
  (`PrimitiveComponent.SetCollisionEnabled` (`/Game/Blueprints/Moving/BP_LivingRoom.Mesh_RoundTable` _returnvalue) "QueryAndPhysics")
  (`PrimitiveComponent.SetCollisionEnabled` (`/Game/Blueprints/Moving/BP_LivingRoom.Mesh_Armchair_02` _returnvalue) "QueryAndPhysics")
  (`PrimitiveComponent.SetCollisionEnabled` (`/Game/Blueprints/Moving/BP_LivingRoom.Mesh_Armchair_03` _returnvalue) "QueryAndPhysics")
  (`PrimitiveComponent.SetCollisionEnabled` (`/Game/Blueprints/Moving/BP_LivingRoom.Mesh_CoffeeTable_02` _returnvalue) "QueryAndPhysics"))

(fn `UserConstructionScript`)