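; BP_HitboxBathroom is a drop zone that reveals the bathroom furniture when a bathroom box is placed in it.
; When its Box begins overlapping a BP_BathroomBox, it finds the BP_Bathroom actor by class and makes its whole component hierarchy visible.
; It then destroys the box and enables query and physics collision on the cabinet body, doors and drawers, printing debug messages along the way.
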(event `self.Box.OnComponentBeginOverlap`
  (params (OverlappedComponent :type "PrimitiveComponent Object Reference") (OtherActor :type "Actor Object Reference") (OtherComp :type "PrimitiveComponent Object Reference") (OtherBodyIndex :type Integer) (bFromSweep :type Boolean) (SweepResult :type "HitResult Structure (by ref)"))
  (cast `/Game/Blueprints/Moving/BP_BathroomBox` OtherActor)
  (`KismetSystemLibrary.PrintString` "ITEM PLACED!")
  (bind _returnvalue (`GameplayStatics.GetActorOfClass` "/Game/Blueprints/Moving/BP_Bathroom.BP_Bathroom_C"))
  (`SceneComponent.SetVisibility` (`/Game/Blueprints/Moving/BP_Bathroom.DefaultSceneRoot` _returnvalue) true true)
  (`KismetSystemLibrary.PrintString` "Visibilty changed!")
  (`self.K2_DestroyActor` OtherActor)
  (`PrimitiveComponent.SetCollisionEnabled` (`/Game/Blueprints/Moving/BP_Bathroom.Mesh_Cabinet_01` _returnvalue) "QueryAndPhysics")
  (`PrimitiveComponent.SetCollisionEnabled` (`/Game/Blueprints/Moving/BP_Bathroom.Mesh_Cabinet_DoorLeft_01` _returnvalue) "QueryAndPhysics")
  (`PrimitiveComponent.SetCollisionEnabled` (`/Game/Blueprints/Moving/BP_Bathroom.Mesh_Cabinet_DoorRight_01` _returnvalue) "QueryAndPhysics")
  (`PrimitiveComponent.SetCollisionEnabled` (`/Game/Blueprints/Moving/BP_Bathroom.Mesh_Cabinet_DrawerLeft_01` _returnvalue) "QueryAndPhysics")
  (`PrimitiveComponent.SetCollisionEnabled` (`/Game/Blueprints/Moving/BP_Bathroom.Mesh_Cabinet_DrawerRight_01` _returnvalue) "QueryAndPhysics"))

(fn `UserConstructionScript`)